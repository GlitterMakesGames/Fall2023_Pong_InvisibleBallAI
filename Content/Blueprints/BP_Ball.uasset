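; Physics-driven Pong-style ball that launches along -X and, past either end of the court, asks BP_BallSpawn for a replacement and destroys itself.
; Paddle hits add an X impulse away from that paddle, gated by CanAccelerate.
; A player-paddle hit also spawns a clone that runs ahead at boosted velocity and self-destroys at its own X bounds.
; The Reveal input toggles clone visibility.
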(event EventBeginPlay
  (Input|EnableInput (Game|GetPlayerController 0))
  (Physics|AddImpulse (Variables|Default|GetSphere) "-10000.000000, 0,0.000000" "None" false))

(event Collision|EventActorBeginOverlap
  (params (OtherActor :type Actor%20Object%20Reference)))

(event EventTick
  (params (DeltaSeconds :type Float%20%28single-precision%29))
  (bind _sphere (Variables|Default|GetSphere))
  (bind _sphere_2 (Variables|Default|GetSphere))
  (bind _returnvalue (Transformation|GetWorldLocation _sphere))
  (bind _returnvalue_2 (Transformation|GetWorldLocation _sphere_2))
  (if (Variables|Default|GetisClone)
    (if (>= (.x _returnvalue) 8e+02)
      (Actor|DestroyActor)
      (elif (<= (.x _returnvalue) -1015.0)
        (Actor|DestroyActor)))
    (elif (<= (.x _returnvalue_2) -1015.0)
      (bind _returnvalue_3 (Actor|GetActorOfClass "/Game/Blueprints/BP_BallSpawn.BP_BallSpawn_C" :!label _label))
      (Default|SpawnBall _returnvalue_3)
      (Actor|DestroyActor)
      (elif (>= (.x _returnvalue_2) 1015.0)
        (goto _label)))))

(event Collision|EventHit
  (params (MyComp :type Primitive%20Component%20Object%20Reference) (Other :type Actor%20Object%20Reference) (OtherComp :type Primitive%20Component%20Object%20Reference) (bSelfMoved :type Boolean) (HitLocation :type Vector :default "0, 0, 0") (HitNormal :type Vector :default "0, 0, 0") (NormalImpulse :type Vector :default "0, 0, 0") (Hit :type Hit%20Result%20Structure%20%28by%20ref%29))
  (if (Variables|Default|GetcanAccelerate)
    (Variables|Default|SetcanAccelerate false)
    (bind _asbp_enemy_paddle (Utilities|Casting|CastToBP_EnemyPaddle Other)
      (:then
        (if (Utilities|IsValid _asbp_enemy_paddle)
          (Physics|AddImpulse (Variables|Default|GetSphere) (Math|Vector|MakeVector -1e+04 0.0 0.0) "None" false)
          (Utilities|FlowControl|Delay 1.0)
          (Variables|Default|SetcanAccelerate true)
          (else
            (bind _asbp_player_paddle (Utilities|Casting|CastToBP_PlayerPaddle Other :!label _label))
            (if (Utilities|IsValid _asbp_player_paddle)
              (Physics|AddImpulse (Variables|Default|GetSphere) (Math|Vector|MakeVector 1e+04 0.0 0.0) "None" false)
              (if (not (Variables|Default|GetisClone))
                (bind _returnvalue (Game|SpawnActorfromClass "BP_Ball_C" (Transformation|GetWorldTransform (Variables|Default|GetSphere)) "Undefined" 0 0))
                (Variables|BP_Ball_C|SetisClone _returnvalue true)
                (Rendering|SetActorHiddenInGame _returnvalue (Variables|Default|GetisHidden))
                (Utilities|FlowControl|Delay 0.2)
                (Physics|SetPhysicsLinearVelocity (Variables|BP_Ball_C|GetSphere _returnvalue) (* (Transformation|GetComponentVelocity (Variables|Default|GetSphere)) 1.25) false "None")
                (Utilities|FlowControl|Delay 1.0)
                (Variables|Default|SetcanAccelerate true))))))
      (:CastFailed
        (goto _label)))))

(event Input|ActionEvents|InputActionReveal
  (params (Key :type Key%20Structure :default "None"))
  (:Pressed
    (if (Variables|Default|GetisClone)
      (if (Variables|Default|GetisHidden)
        (bind _output_get (Variables|Default|SetisHidden false))
        (Rendering|SetActorHiddenInGame _output_get)
        (else
          (bind _output_get_2 (Variables|Default|SetisHidden true))
          (Rendering|SetActorHiddenInGame _output_get_2))))))

(event Input|KeyboardEvents|SpaceBar
  (params (Key :type Key%20Structure :default "None")))

(fn ConstructionScript)