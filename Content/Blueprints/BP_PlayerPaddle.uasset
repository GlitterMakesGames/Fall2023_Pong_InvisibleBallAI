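; BP_PlayerPaddle is a player-controlled paddle that moves vertically between fixed upper and lower limits.
; Each Tick offsets the Cube component along local Z by an input axis key value times Speed2.
; When the Cube's world height, padded by a fixed margin, passes a limit, a constant nudge back inward replaces input.
; Movement is per frame, without delta-time scaling.
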(event EventBeginPlay
  (|CallParentFunction) ; This node is disabled and will not be called.\nDrag off pins to build functionality.
)

(event Collision|EventActorBeginOverlap
  (params (OtherActor :type Actor%20Object%20Reference))
  (|CallParentFunction OtherActor) ; This node is disabled and will not be called.\nDrag off pins to build functionality.
)

(event EventTick
  (params (DeltaSeconds :type Float%20%28single-precision%29))
  (bind _cube (Variables|Default|GetCube))
  (bind _cube_2 (Variables|Default|GetCube))
  (bind _returnvalue (Transformation|GetWorldLocation _cube_2))
  (|CallParentFunction DeltaSeconds)
  (if (<= (+ (.z _returnvalue) 5e+01) 6e+02)
    (if (>= (- (.z _returnvalue) 5e+01) -375.0)
      (Transformation|AddLocalOffset (Variables|Default|GetCube) (Math|Vector|MakeVector 0.0 0.0 (* (Class|Actor|GetInputAxisKeyValue) (Variables|Default|GetSpeed2))) false false)
      (else
        (Transformation|AddLocalOffset _cube (Math|Vector|MakeVector 0.0 0.0 1e+01) false false)))
    (else
      (Transformation|AddLocalOffset _cube (Math|Vector|MakeVector 0.0 0.0 -1e+01) false false))))

(fn ConstructionScript
  (|CallParentFunction))