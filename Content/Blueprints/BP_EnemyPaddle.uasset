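; BP_EnemyPaddle is an AI-controlled paddle that moves its Cube vertically to follow a ball.
; Each tick it searches all BP_Ball actors, stopping at the first flagged IsClone, and uses that loop index as the target.
; MoveComponentTo eases the Cube toward the target's Z over MoveTime, while fixed offsets nudge it back inside hard-coded height limits.
; A tag-based clone lookup is left unconnected.
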(event EventBeginPlay
  (|CallParentFunction) ; This node is disabled and will not be called.\nDrag off pins to build functionality.
)

(event Collision|EventActorBeginOverlap
  (params (OtherActor :type Actor%20Object%20Reference))
  (|CallParentFunction OtherActor) ; This node is disabled and will not be called.\nDrag off pins to build functionality.
)

(event EventTick
  (params (DeltaSeconds :type Float%20%28single-precision%29))
  (bind _cube (Variables|Default|GetCube))
  (bind _cube_2 (Variables|Default|GetCube))
  (bind _returnvalue (Transformation|GetWorldLocation _cube))
  (|CallParentFunction DeltaSeconds)
  (bind _outactors (Actor|GetAllActorsOfClass "/Game/Blueprints/BP_Ball.BP_Ball_C"))
  (bind (_array_element _array_index) (Utilities|Array|ForEachLoopwithBreak _outactors :!label _label)
    (:LoopBody
      (Variables|Default|SetArrayIndex _array_index)
      (if (Variables|/Game/Blueprints/BP_Ball.BP_Ball_C|GetisClone _array_element)
        (goto _label Break)))
    (:Completed
      (if (!= (Utilities|Array|Get(acopy) _outactors (Variables|Default|GetArrayIndex)) 0)
        (if (<= (+ (.z _returnvalue) 5e+01) 6e+02)
          (if (>= (- (.z _returnvalue) 5e+01) -375.0)
            (Components|MoveComponentTo _cube (Math|Vector|MakeVector 0.0 0.0 (.z (Transformation|GetActorLocation (Utilities|Array|Get(acopy) _outactors (Variables|Default|GetArrayIndex))))) "0, 0, 0" false false (Variables|Default|GetMoveTime) false)
            (else
              (Transformation|AddLocalOffset _cube_2 (Math|Vector|MakeVector 0.0 0.0 1e+01) false false)))
          (else
            (Transformation|AddLocalOffset _cube_2 (Math|Vector|MakeVector 0.0 0.0 -1e+01) false false)))))))

(fn ConstructionScript
  (|CallParentFunction))